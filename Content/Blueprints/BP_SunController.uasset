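; Sun controller actor that sets the Sunlight's pitch from the system clock.
; BeginPlay applies the rotation, starts a looping timer with no function name shown, and recaptures the Skylight once.
; UpdateSunRotation maps 6:00–18:00 onto a clamped pitch lerp at fixed yaw.
; The time math divides integers before converting to double, so pitch jumps between its endpoints instead of sweeping.
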(event Custom|UpdateSunRotation
  (bind _returnvalue (Math|DateTime|Now))
  (bind (_year _month _day _hour _minute) (Math|DateTime|BreakDateTime _returnvalue))
  (bind _output_get (Variables|Default|SetReturn%20Value%20Minute _minute))
  (bind _output_get_2 (Variables|Default|SetReturn%20Value%20Hour _hour))
  (Transformation|SetActorRotation (Variables|Default|GetSunlight) (Math|Rotator|MakeRotator 0.0 (Math|Float|Lerp -1e+01 45.0 (Math|Float|Clamp(Float) (Math|Conversions|ToFloat(Integer) (/ (- (+ _output_get_2 (/ _output_get 60)) 6) 12)))) 9e+01)))

(event Collision|EventActorBeginOverlap
  (params (OtherActor :type Actor%20Object%20Reference)))

(event EventTick
  (params (DeltaSeconds :type Float%20%28single-precision%29)))

(event EventBeginPlay
  (CallFunction|UpdateSunRotation)
  (Utilities|Time|SetTimerbyFunctionName 0 "" 0.6 true)
  (Class|SkyLightComponent|RecaptureSky (Variables|/Script/Engine.SkyLight|GetLightComponent (Variables|Default|GetSkylight))))

(fn ConstructionScript)