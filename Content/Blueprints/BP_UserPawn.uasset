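; BP_UserPawn is the player pawn that sets up the fixed camera view and user interface at game start.
; On BeginPlay it switches the view to the first CameraActor found in the level.
; It then creates WBP_UserHUD with the IamaiVoiceInput reference, adds it to the viewport, and sets UI-only input focused on the HUD with a visible cursor.
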(event EventBeginPlay
  (Utilities|FlowControl|Sequence
    (:then_0
      (bind _returnvalue (Actor|GetActorOfClass "/Script/Engine.CameraActor"))
      (Game|Player|SetViewTargetwithBlend (Game|GetPlayerController 0) _returnvalue 0.0 "VTBlend_Linear" 0.0 false))
    (:then_1
      (bind _returnvalue_2 (UserInterface|CreateWidget "/Game/UI/WBP_UserHUD.WBP_UserHUD_C" 0 (Variables|Default|GetiamaiVoiceInput)))
      (bind _output_get (Variables|Default|SetHUD _returnvalue_2))
      (UserInterface|Viewport|AddtoViewport _output_get 0))
    (:then_2
      (Input|SetInputModeUIOnly (Game|GetPlayerController 0) (Variables|Default|GetHUD) "DoNotLock" true)
      (Variables|/Script/Engine.PlayerController|SetbShowMouseCursor (Game|GetPlayerController 0) true))))

(fn ConstructionScript)